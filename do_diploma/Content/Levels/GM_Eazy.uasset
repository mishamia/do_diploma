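; GM_Eazy, likely the game mode for an easy level, spawns a square grid of Yzel actors when play begins.
; BeginPlay fills the LocYzli array with evenly spaced 10×10 positions on the XY plane, starting at the world origin.
; It then calls SpawnsYzli, which spawns one Yzel at each stored location.
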(event EventBeginPlay
  (for _index (range 0 9)
    (for _index_2 (range 0 9)
      (Utilities|Array|AddUnique (Variables|Default|GetLoc_Yzli) (+ (* "25.000000, 0, 0" _index) (* "0,25.000000, 0" _index_2)))))
  (CallFunction|SpawnsYzli))

(event EventTick
  (params (DeltaSeconds :type Float%20%28single-precision%29)))

(fn ConstructionScript)

(fn SpawnsYzli
  (for _index (range 0 99)
    (Game|SpawnActorfromClass "/Game/Levels/Yzel.Yzel_C" (Math|Transform|MakeTransform (Utilities|Array|Get(acopy) (Variables|Default|GetLoc_Yzli) _index) "0, 0, 0" "1,1,1") "Undefined" 0 0)))